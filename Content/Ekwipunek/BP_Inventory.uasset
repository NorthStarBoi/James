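; BP_Inventory is an inventory component for BP_BaseCharacter that stores items and their images in two parallel arrays.
; Add and Remove update both arrays, print the item, then cast the owner to reach its InventoryWidget.
; Both call AddItemToListUI, so removal also sends an add to the UI.
; CheckInventory loops over items but returns only the final comparison, so it effectively tests the last entry.
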(event EventBeginPlay)

(event EventTick
  (params (DeltaSeconds :type Float%20%28single-precision%29)))

(fn AddItemtoInventory
  (params (NewItem :type String%20%28by%20ref%29) (NewItem1 :type Texture%202D%20Object%20Reference%20%28by%20ref%29))
  (Utilities|Array|Add (Variables|Default|GetInventory) NewItem)
  (Utilities|Array|Add (Variables|Default|GetImage) NewItem1)
  (Development|PrintString NewItem)
  (bind _asbp_base_character (Utilities|Casting|CastToBP_BaseCharacter (Components|GetOwner)))
  (Default|AddItemtoListUI (Variables|/Game/ThirdPerson/Blueprints/BP_BaseCharacter.BP_BaseCharacter_C|GetInventory%20Widget _asbp_base_character) NewItem NewItem1))

(fn CheckInventory
  (params (RequiredItem :type String))
  (for _array_element (Variables|Default|GetInventory)
    (if (Utilities|Enum|Equal(Enum) RequiredItem _array_element)
      _))
  (return (Utilities|Enum|Equal(Enum) RequiredItem _array_element)))

(fn RemoveItemfromInventory
  (params (Item :type String%20%28by%20ref%29) (Item1 :type Texture%202D%20Object%20Reference%20%28by%20ref%29))
  (Utilities|Array|RemoveItem (Variables|Default|GetInventory) Item)
  (Utilities|Array|RemoveItem (Variables|Default|GetImage) Item1)
  (Development|PrintString Item)
  (bind _asbp_base_character (Utilities|Casting|CastToBP_BaseCharacter (Components|GetOwner)))
  (Default|AddItemtoListUI (Variables|/Game/ThirdPerson/Blueprints/BP_BaseCharacter.BP_BaseCharacter_C|GetInventory%20Widget _asbp_base_character) Item Item1))