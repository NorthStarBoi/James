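; BP_Locker is an interactable locker that shows an interaction prompt and outline, though its Interact event is still empty.
; When CanInteract is set, sphere overlap registers it as the character's TraceItem, spawns UI_Interact, plays PopUp and applies M_Outline.
; End overlap clears TraceItem, reverses the animation and removes the widget, but reapplies the outline instead of clearing it.
; CanRecieveTrace also drives the prompt, outline and CanPressE flag.
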(event OnComponentBeginOverlap(Sphere)
  (params (OverlappedComponent :type Primitive%20Component%20Object%20Reference) (OtherActor :type Actor%20Object%20Reference) (OtherComp :type Primitive%20Component%20Object%20Reference) (OtherBodyIndex :type Integer) (bFromSweep :type Boolean) (SweepResult :type Hit%20Result%20Structure%20%28by%20ref%29))
  (bind __widget (Variables|Default|Get%20Widget))
  (bind _asbp_base_character (Utilities|Casting|CastToBP_BaseCharacter OtherActor))
  (if (Variables|Default|GetCanInteract)
    (Variables|/Game/ThirdPerson/Blueprints/BP_BaseCharacter.BP_BaseCharacter_C|SetTraceItem _asbp_base_character self)
    (bind _returnvalue (UserInterface|CreateWidget "/Game/Interakcje/UI_Interact.UI_Interact_C"))
    (bind _output_get (Variables|Default|SetInterActionWidget _returnvalue))
    (UserInterface|SetWidget __widget _output_get)
    (Rendering|SetVisibility __widget true false)
    (bind _interactionwidget (Variables|Default|GetInterActionWidget)
      (:then
        (if (not (Variables|Default|GetHintVisible))
          (UserInterface|Animation|PlayAnimation _interactionwidget (Variables|/Game/Interakcje/UI_Interact.UI_Interact_C|GetPopUp _interactionwidget) 0.0 1 "Forward" 1.5 false)
          (Variables|Default|SetHintVisible true)
          (Rendering|Material|SetOverlayMaterial (Variables|Default|GetStaticMesh) "/Game/Interakcje/M_Outline.M_Outline" :!class /Script/Engine.MeshComponent)
          (Variables|Default|SetCanPressE true)))
      (:else))))

(event OnComponentEndOverlap(Sphere)
  (params (OverlappedComponent :type Primitive%20Component%20Object%20Reference) (OtherActor :type Actor%20Object%20Reference) (OtherComp :type Primitive%20Component%20Object%20Reference) (OtherBodyIndex :type Integer))
  (bind _asbp_base_character (Utilities|Casting|CastToBP_BaseCharacter OtherActor))
  (if (Variables|Default|GetCanInteract)
    (Variables|/Game/ThirdPerson/Blueprints/BP_BaseCharacter.BP_BaseCharacter_C|SetTraceItem _asbp_base_character 0)
    (bind _interactionwidget (Variables|Default|GetInterActionWidget)
      (:then
        (if (Variables|Default|GetHintVisible)
          (UserInterface|Animation|PlayAnimation _interactionwidget (Variables|/Game/Interakcje/UI_Interact.UI_Interact_C|GetPopUp _interactionwidget) 0.0 1 "Reverse" 1.5 false)
          (Variables|Default|SetHintVisible false)
          (Variables|Default|SetCanPressE false)
          (Rendering|Material|SetOverlayMaterial (Variables|Default|GetStaticMesh) "/Game/Interakcje/M_Outline.M_Outline" :!class /Script/Engine.MeshComponent))
        (Utilities|FlowControl|Delay 0.15)
        (Widget|RemovefromParent (Variables|Default|GetInterActionWidget))
        (Variables|Default|SetInterActionWidget 0)
        (Rendering|SetVisibility (Variables|Default|Get%20Widget) false false))
      (:else))))

(event EventCanRecieveTrace
  (params (CanInteract :type Boolean))
  (if (Variables|Default|GetCanInteract)
    (if CanInteract
      (bind _interactionwidget (Variables|Default|GetInterActionWidget)
        (:then
          (if (Variables|Default|GetHintVisible)
            _
            (else
              _))
          (UserInterface|Animation|PlayAnimation _interactionwidget (Variables|/Game/Interakcje/UI_Interact.UI_Interact_C|GetPopUp _interactionwidget) 0.0 1 "Forward" 1.5 false)
          (Variables|Default|SetHintVisible true)
          (Rendering|Material|SetOverlayMaterial (Variables|Default|GetStaticMesh) "/Game/Interakcje/M_Outline.M_Outline" :!class /Script/Engine.MeshComponent)
          (Variables|Default|SetCanPressE true))
        (:else))
      (else
        (bind _interactionwidget_2 (Variables|Default|GetInterActionWidget)
          (:then
            (if (not (Variables|Default|GetHintVisible))
              (UserInterface|Animation|PlayAnimation _interactionwidget_2 (Variables|/Game/Interakcje/UI_Interact.UI_Interact_C|GetPopUp _interactionwidget_2) 0.0 1 "Reverse" 1.5 false)
              (Variables|Default|SetHintVisible false)
              (Rendering|Material|SetOverlayMaterial (Variables|Default|GetStaticMesh) 0 :!class /Script/Engine.MeshComponent)
              (Variables|Default|SetCanPressE false)))
          (:else))))))

(event EventInteract)

(fn ConstructionScript)